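; Player controller that registers the Enhanced Input mapping context on BeginPlay and routes player input to the controlled pawn.
; Camera input is applied directly as pitch and yaw after a pawn validity check.
; Move, shoot, boost and aim are sent as messages, decoupling the controller from the pawn class.
; Boost and aim share one path for Started and Completed, forwarding only when the action value is false.
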(event Input|EnhancedActionEvents|EnhancedInputActionShoot_IA
  (params (ActionValue :type Boolean) (ElapsedSeconds :type Float%20%28double-precision%29) (TriggeredSeconds :type Float%20%28double-precision%29) (InputAction :type Input%20Action%20Object%20Reference :default "/Game/PlayerInputs/Shoot_IA.Shoot_IA"))
  (:Triggered
    (Class|PlayerInputBPI|PlayerShoot(Message) (Pawn|GetControlledPawn))))

(event Input|EnhancedActionEvents|EnhancedInputActionBoost_IA
  (params (ActionValue :type Boolean) (ElapsedSeconds :type Float%20%28double-precision%29) (TriggeredSeconds :type Float%20%28double-precision%29) (InputAction :type Input%20Action%20Object%20Reference :default "/Game/PlayerInputs/Boost_IA.Boost_IA"))
  (:Started
    (if (not (stale Input|EnhancedActionEvents|EnhancedInputActionAim_IA ActionValue)) :!label _label
      (Class|PlayerInputBPI|PlayerBoost(Message) (Pawn|GetControlledPawn) ActionValue)))
  (:Completed
    (goto _label)))

(event Input|EnhancedActionEvents|EnhancedInputActionMove_IA
  (params (ActionValue :type Vector%202D%20Structure) (ElapsedSeconds :type Float%20%28double-precision%29) (TriggeredSeconds :type Float%20%28double-precision%29) (InputAction :type Input%20Action%20Object%20Reference :default "/Game/PlayerInputs/Move_IA.Move_IA"))
  (:Triggered
    (Class|PlayerInputBPI|PlayerMovement(Message) (Pawn|GetControlledPawn) ActionValue)))

(event Input|EnhancedActionEvents|EnhancedInputActionAim_IA
  (params (ActionValue :type Boolean) (ElapsedSeconds :type Float%20%28double-precision%29) (TriggeredSeconds :type Float%20%28double-precision%29) (InputAction :type Input%20Action%20Object%20Reference :default "/Game/PlayerInputs/Aim_IA.Aim_IA"))
  (:Started
    (if (not (stale Input|EnhancedActionEvents|EnhancedInputActionBoost_IA ActionValue)) :!label _label
      (Class|PlayerInputBPI|PlayerAim(Message) (Pawn|GetControlledPawn) ActionValue)))
  (:Completed
    (goto _label)))

(event Input|EnhancedActionEvents|EnhancedInputActionCameraControl_IA
  (params (ActionValue :type Vector%202D%20Structure) (ElapsedSeconds :type Float%20%28double-precision%29) (TriggeredSeconds :type Float%20%28double-precision%29) (InputAction :type Input%20Action%20Object%20Reference :default "/Game/PlayerInputs/CameraControl_IA.CameraControl_IA"))
  (bind _returnvalue (Pawn|GetControlledPawn))
  (bind (_x _y) (Math|Vector2D|BreakVector2D ActionValue))
  (:Triggered
    (Utilities|IsValid _returnvalue
      (:Is%20Valid
        (Pawn|Input|AddControllerPitchInput _returnvalue _x)
        (Pawn|Input|AddControllerYawInput _returnvalue _y)))))

(event EventBeginPlay
  (Input|AddMappingContext (PlayerController|LocalPlayerSubsystems|GetEnhancedInputLocalPlayerSubsystem) "/Game/PlayerInputs/PlayerInputContext.PlayerInputContext" 0 "(bIgnoreAllPressedKeysUntilRelease=True,bForceImmediately=False)"))

(event EventTick
  (params (DeltaSeconds :type Float%20%28single-precision%29)))

(fn ConstructionScript)