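; Player HUD that creates the PlayerUI_BP widget at BeginPlay and marks enemies on screen with reticles.
; Each frame it draws a translucent red selection rectangle and queries it for EnemyPH_BP actors.
; Those within a set distance band from the controlled pawn get Reticle_M drawn centered on their projected screen position.
; CalculateScreenForActorSelection supplies the rectangle origin, though its graph holds only unconnected viewport-centering math.
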(event EventBeginPlay
  (bind _returnvalue (UserInterface|CreateWidget "/Game/PlayerUI/PlayerUI_BP.PlayerUI_BP_C" (Game|Player|GetOwningPlayerController)))
  (UserInterface|Viewport|AddtoViewport _returnvalue 0))

(event Collision|EventActorBeginOverlap
  (params (OtherActor :type Actor%20Object%20Reference)))

(event EventTick
  (params (DeltaSeconds :type Float%20%28single-precision%29)))

(event EventDrawHUD
  (params (SizeX :type Integer) (SizeY :type Integer))
  (bind _returnvalue (Game|Player|GetOwningPlayerController))
  (bind (_screenx _screeny) (Utilities|CalculateScreenforActorSelection))
  (bind (_screenx_2 _screeny_2) (Utilities|CalculateScreenforActorSelection))
  (bind _screenpixelwidth (Variables|Default|GetScreenPixelWidth))
  (bind _screenpixelheigth (Variables|Default|GetScreenPixelHeigth))
  (HUD|DrawRect "(R=0.614583,G=0.006631,B=0.000000,A=0.100000)" _screenx _screeny _screenpixelwidth _screenpixelheigth)
  (for _array_element (Class|HUD|GetActorsinSelectionRectangle "/Game/Enemy/EnemyPH_BP.EnemyPH_BP_C" (Math|Vector2D|MakeVector2D _screenx_2 _screeny_2) (Math|Vector2D|MakeVector2D _screenpixelwidth _screenpixelheigth) false false)
    (if (Math|Float|InRange(Float) (Transformation|GetDistanceTo (Pawn|GetControlledPawn _returnvalue) _array_element) 2e+03 2e+04)
      (Class|HUD|DrawMaterialSimple "/Game/Texture/Reticle_M.Reticle_M" (- (.x (.ScreenPosition (Class|GameplayStatics|ProjectWorldtoScreen _returnvalue (Transformation|GetActorLocation _array_element) true))) 2e+01) (- (.y (.ScreenPosition (Class|GameplayStatics|ProjectWorldtoScreen _returnvalue (Transformation|GetActorLocation _array_element) true))) 2e+01) 4e+01 4e+01 1.0 true))))

(fn ConstructionScript)