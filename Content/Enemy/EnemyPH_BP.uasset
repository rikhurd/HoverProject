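; Enemy Blueprint that turns to face actors it sees and switches to physics simulation when damaged.
; Taking damage enables physics on the capsule and sets a five-second timer by function name, restarted by further hits while it exists, apparently to call ResetPhysicsSimulation.
; While physics is off, Tick snaps rotation toward each actor perceived by AI sight, leaving it facing the last one.
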(event Custom|OnTakeAnyDamage_Event
  (params (DamagedActor :type Actor%20Object%20Reference) (Damage :type Float%20%28single-precision%29) (DamageType :type Damage%20Type%20Object%20Reference) (InstigatedBy :type Controller%20Object%20Reference) (DamageCauser :type Actor%20Object%20Reference))
  (bind _capsulecomponent (Variables|Collision|GetCapsuleComponent))
  (if (Class|SceneComponent|IsAnySimulatingPhysics _capsulecomponent)
    (if (Class|KismetSystemLibrary|TimerExistsHandle (stale _returnvalue))
      (bind _returnvalue (Utilities|Time|SetTimerbyFunctionName 0 (Variables|Default|GetResetPhysicsFunctionName) 5.0 :!label _label)))
    (else
      (CallFunction|SettoSimulatePhysics _capsulecomponent true)
      (goto _label))))

(event EventBeginPlay
  (EventDispatchers|BindEventtoOnTakeAnyDamage (delegate Custom|OnTakeAnyDamage_Event)))

(event Collision|EventActorBeginOverlap
  (params (OtherActor :type Actor%20Object%20Reference)))

(event EventTick
  (params (DeltaSeconds :type Float%20%28single-precision%29))
  (if (not (Class|SceneComponent|IsAnySimulatingPhysics (Variables|Collision|GetCapsuleComponent)))
    (for _array_element (Class|AIPerceptionComponent|GetCurrentlyPerceivedActors (Variables|Default|GetAIPerception) "/Script/AIModule.AISense_Sight")
      (Transformation|SetActorRotation (Math|Rotator|FindLookatRotation (Transformation|GetActorLocation) (Transformation|GetActorLocation _array_element))))))

(fn ConstructionScript)

(fn SettoSimulatePhysics
  (params (PrimitiveComponent :type Primitive%20Component%20Object%20Reference) (bSimulatePhysics :type Boolean))
  (bind _output_get (Variables|Default|SetbSimulatePhysics bSimulatePhysics))
  (Physics|SetSimulatePhysics PrimitiveComponent _output_get))

(fn ResetPhysicsSimulation
  (CallFunction|SettoSimulatePhysics (Variables|Collision|GetCapsuleComponent) false))