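; Player vehicle weapon with an area-damage shot and a toggleable physics grappling cable.
; Shooting traces from barrel toward camera aim, adds recoil to the vehicle, then applies radial damage, impulses and impact VFX.
; The cable capsule-traces from the camera and spawns a constraint actor between vehicle and target, ordering components and scaling length by target class.
; Enemy physics simulation toggles for dragging; lock-on box search is unwired.
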(event EventPlayerCable
  (params (isShot :type Boolean))
  (bind _radius (Variables|Default|GetRadius))
  (bind _camera (Variables|Default|GetCamera))
  (bind _radius_2 (Variables|Default|GetRadius))
  (bind _cablehitcomponent (Variables|Default|GetCableHitComponent))
  (bind _cable (Variables|Default|GetCable))
  (bind _cablehitcomponent_2 (Variables|Default|GetCableHitComponent))
  (bind _physicsconstraintref (Variables|Default|GetPhysicsConstraintRef))
  (bind _returnvalue (Math|Vector|GetForwardVector _camera))
  (bind _returnvalue_2 (Transformation|GetWorldLocation _camera))
  (bind _constraintcomp (Variables|/Script/Engine.PhysicsConstraintActor|GetConstraintComp _physicsconstraintref))
  (if (Variables|Default|GetbCableConnected)
    (Variables|Default|SetbCableConnected false)
    (Rendering|SetVisibility (Variables|Default|GetCable) false false)
    (Utilities|FlowControl|Sequence
      (:then_0
        (Utilities|IsValid _constraintcomp
          (:Is%20Valid
            (Class|PhysicsConstraintComponent|BreakConstraint _constraintcomp)
            (Actor|DestroyActor (Variables|Default|GetPhysicsConstraintRef)))))
      (:then_1
        (Utilities|IsValid _cablehitcomponent
          (:Is%20Valid
            (CallFunction|SettoSimulatePhysics (Physics|IsSimulatingPhysics _cablehitcomponent (Variables|Default|GetCableHitBoneName)) _cablehitcomponent)
            (Class|PrimitiveComponent|SetNotifyRigidBodyCollision (Variables|Default|GetCableHitComponent) false)
            (Development|PrintString "Cable constraint has broken")))))
    (else
      (bind _returnvalue_3 (Niagara|SpawnSystemAttached "/Game/WP_PH/VFX/WeaponShoot_VFX.WeaponShoot_VFX" (Variables|Default|GetSkeletalMesh) "Barrel" "0, 0, 0" "0, 0, 0" "KeepWorldPosition" true true "AutoRelease"))
      (Niagara|SetNiagaraVariable(Vector3) _returnvalue_3 "BeamEndVector" "0, 0, 0")
      (bind (_outhit _returnvalue_4) (Collision|CapsuleTraceByChannel (+ _returnvalue_2 (* _returnvalue (+ _radius_2 _radius_2))) (+ _returnvalue_2 (* _returnvalue (Variables|Default|GetWeaponLineTraceModifier))) _radius _radius "TraceTypeQuery1" false (Utilities|Array|MakeArray (Components|GetOwner)) "ForDuration" true "(R=1.000000,G=0.271195,B=0.029739,A=1.000000)"))
      (if _returnvalue_4
        (CallFunction|SetCableHitVariables (.Distance (Collision|BreakHitResult _outhit)) (.HitActor (Collision|BreakHitResult _outhit)) (.HitComponent (Collision|BreakHitResult _outhit)) (.HitBoneName (Collision|BreakHitResult _outhit))) ; Sets Hit Variables for organizing BP
        (Variables|Default|SetbCableConnected true)
        (Variables|/Script/CableComponent.CableComponent|SetCableLength _cable (Variables|Default|GetCableHitDistance))
        (Rendering|SetVisibility _cable true false)
        (Class|CableComponent|SetAttachEndto _cable (Variables|Default|GetCableHitActor) "None" (Variables|Default|GetCableHitBoneName))
        (if (CallFunction|CheckHitActorisEnemy)
          (Utilities|FlowControl|Sequence
            (:then_0
              ;[1 1 1] If Hit Actor is suitable to drag around by player set it to simulate physics
              (CallFunction|SettoSimulatePhysics (Physics|IsSimulatingPhysics _cablehitcomponent_2 (Variables|Default|GetCableHitBoneName)) _cablehitcomponent_2))
            (:then_1
              ;[1 1 1] Set physics constraint between player and hit Actor
              (bind _hitdistanceout (CallFunction|SetContraintComponEnemyHit (Variables|Default|GetCableHitComponent) (Variables|Default|GetCableHitBoneName) (Variables|Default|GetCableHitActor) (Variables|Default|GetCableHitDistance) :!label _label))
              (CallFunction|SetConstraintLimit _hitdistanceout)))
          (else
            (goto _label)))))))

(event EventBeginPlay
  ;[1 1 1] Cast to player vehicle to get camera for line trace and mesh for impulse
  (bind _asplayer_vehicle_bp (Utilities|Casting|CastToPlayerVehicle_BP (Components|GetOwner)))
  (Variables|Default|SetCamera (Variables|/Game/PlayerCharacter/PH_Model/BP/PlayerVehicle_BP.PlayerVehicle_BP_C|GetThirdPersonCamera _asplayer_vehicle_bp))
  (Variables|Default|SetAs%20Player%20Vehicle%20BP _asplayer_vehicle_bp))

(event EventPlayerShoot
  (bind _camera (Variables|Default|GetCamera))
  (bind _weaponlinetracemodifier (Variables|Default|GetWeaponLineTraceModifier))
  (bind _returnvalue (Math|Vector|GetForwardVector _camera))
  (bind _returnvalue_2 (Transformation|GetWorldLocation _camera))
  (bind _returnvalue_3 (* _returnvalue _weaponlinetracemodifier))
  (bind _returnvalue_4 (+ _returnvalue_2 _returnvalue_3))
  (bind (_outhit _returnvalue_5) (Collision|LineTraceByChannel (Transformation|GetSocketLocation (Variables|Default|GetSkeletalMesh) "Barrel") _returnvalue_4 "TraceTypeQuery1" false (Utilities|Array|MakeArray (Components|GetOwner)) "None" true "(R=1.000000,G=0.000000,B=0.000000,A=1.000000)" "(R=0.000000,G=1.000000,B=0.000000,A=1.000000)" 2.0))
  ;[1 1 1] Add recoil on shooting
  (Physics|AddImpulseatLocation (Variables|/Game/PlayerCharacter/PH_Model/BP/PlayerVehicle_BP.PlayerVehicle_BP_C|GetVehicleMesh (Variables|Default|GetAs%20Player%20Vehicle%20BP)) (- (Transformation|GetSocketLocation (Variables|Default|GetSkeletalMesh) "Barrel") (* (Math|Vector|GetForwardVector (Variables|Default|GetSkeletalMesh)) (Variables|Default|GetWeaponRecoilMultiplier))) (Transformation|GetWorldLocation (Variables|/Script/Engine.Actor|GetRootComponent (Variables|Default|GetAs%20Player%20Vehicle%20BP))) "None")
  (bind _output_get (Variables|Default|SetBulletStopLocation (Math|Vector|Lerp(Vector) _returnvalue_4 (.Location (Collision|BreakHitResult _outhit)) (Math|Conversions|ToFloat(Boolean) _returnvalue_5))))
  ;[1 1 1] Create sphere where line trace hit to modify later
  (bind (_outcomponents _returnvalue_6) (Collision|SphereOverlapComponents _output_get (Variables|Components|GetBulletRadius) (Utilities|Array|MakeArray "ObjectTypeQuery4" "ObjectTypeQuery7" "ObjectTypeQuery6") "/Script/Engine.PrimitiveComponent"))
  (if _returnvalue_6
    ;[1 1 1] Apply physic force and damage to caught objects
    (bind _returnvalue_7 (Game|Damage|ApplyRadialDamage (Variables|Default|GetWeaponDamage) (Variables|Default|GetBulletStopLocation) (Variables|Components|GetBulletRadius) "/Game/WP_PH/BP/PlayerWeaponDamageType_BP.PlayerWeaponDamageType_BP_C" 0 (Components|GetOwner) 0 true "ECC_Visibility"))
    (if _returnvalue_7
      (for _array_element _outcomponents
        (Physics|AddRadialImpulse _array_element (Variables|Default|GetBulletStopLocation) (Variables|Components|GetBulletRadius) (Variables|Default|GetWeaponImpulseStrength) "RIF_Linear" false)
        (Class|PrimitiveComponent|AddAngularImpulseinDegrees _array_element (* (Math|Vector|NegateVector (Variables|Default|GetBulletStopLocation)) (/ (Variables|Default|GetWeaponImpulseStrength) 2.0)) "None" false))))
  (if _returnvalue_5
    (Niagara|SpawnSystematLocation "/Game/WP_PH/VFX/AmmoImpact_VFX.AmmoImpact_VFX" (.Location (Collision|BreakHitResult _outhit)) (Math|Rotator|FindLookatRotation (+ (.Location (Collision|BreakHitResult _outhit)) (.Normal (Collision|BreakHitResult _outhit))) (.Normal (Collision|BreakHitResult _outhit))) "1.000000,1.000000,1.000000" true true "AutoRelease")))

(fn ConstructionScript)

(fn SetConstraintLimit
  (params (Distance :type Float%20%28double-precision%29))
  (bind _physicsconstraintref (Variables|Default|GetPhysicsConstraintRef))
  (bind _constraintcomp (Variables|/Script/Engine.PhysicsConstraintActor|GetConstraintComp _physicsconstraintref))
  (Class|PhysicsConstraintComponent|SetLinearXLimit _constraintcomp "LCM_Limited" Distance)
  (Class|PhysicsConstraintComponent|SetLinearYLimit _constraintcomp "LCM_Limited" Distance)
  (Class|PhysicsConstraintComponent|SetLinearZLimit _constraintcomp "LCM_Limited" Distance))

(fn SetContraintComponEnemyHit
  (params (HitComponent :type Primitive%20Component%20Object%20Reference) (HitBoneName :type Name) (HitActor :type Actor%20Object%20Reference) (HitDistanceIn :type Float%20%28double-precision%29))
  (bind _as_player_vehicle_bp (Variables|Default|GetAs%20Player%20Vehicle%20BP))
  (bind _vehiclemesh (Variables|/Game/PlayerCharacter/PH_Model/BP/PlayerVehicle_BP.PlayerVehicle_BP_C|GetVehicleMesh _as_player_vehicle_bp))
  (bind _returnvalue (Class|SkinnedMeshComponent|GetSocketBoneName _vehiclemesh "Weapon_Socket"))
  (LocalVariables|SetHitDistance HitDistanceIn)
  (bind _output_get (LocalVariables|SetbPlayerDominates (== (Utilities|GetClass HitActor) "/Game/Enemy/Enemy_BP.Enemy_BP_C"))) ; Orders where physics constraint is placed and constraint's dominating actor
  (if _output_get
    (bind _returnvalue_2 (Game|SpawnActorfromClass "/Game/PlayerCharacter/PH_Model/BP/CableConstraint_BP.CableConstraint_BP_C" (Transformation|GetWorldTransform HitComponent) "Undefined" 0 0))
    (bind _output_get_2 (Variables|Default|SetPhysicsConstraintRef _returnvalue_2))
    (Class|PhysicsConstraintComponent|SetConstrainedComponents (Variables|/Script/Engine.PhysicsConstraintActor|GetConstraintComp _output_get_2) HitComponent HitBoneName _vehiclemesh _returnvalue)
    (Class|PrimitiveComponent|SetNotifyRigidBodyCollision HitComponent true)
    (else
      (bind _returnvalue_3 (Game|SpawnActorfromClass "/Game/PlayerCharacter/PH_Model/BP/CableConstraint_BP.CableConstraint_BP_C" (Transformation|GetSocketTransform (Variables|/Game/PlayerCharacter/PH_Model/BP/PlayerVehicle_BP.PlayerVehicle_BP_C|GetVehicleMesh (Variables|Default|GetAs%20Player%20Vehicle%20BP)) "None" "RTS_World") "Undefined" 0 0))
      (bind _output_get_3 (Variables|Default|SetPhysicsConstraintRef _returnvalue_3))
      (Class|PhysicsConstraintComponent|SetConstrainedComponents (Variables|/Script/Engine.PhysicsConstraintActor|GetConstraintComp _output_get_3) _vehiclemesh _returnvalue HitComponent HitBoneName)
      (LocalVariables|SetHitDistance (* HitDistanceIn (LocalVariables|GetHitDistanceMultiplier)))))
  (return (LocalVariables|GetHitDistance)))

(fn SettoSimulatePhysics
  (params (bSimulatingPhysics :type Boolean) (CableHitComponent :type Primitive%20Component%20Object%20Reference))
  (if bSimulatingPhysics
    (if (Class|KismetSystemLibrary|TimerExists (Variables|Default|GetCableHitActor) (Variables|Default|GetResetPhysicsFunctionName))
      (Utilities|Time|ClearTimerbyFunctionName (Variables|Default|GetCableHitActor) (Variables|Default|GetResetPhysicsFunctionName))
      (else
        (Physics|SetSimulatePhysics (Variables|Default|GetCableHitComponent) false)))
    (else
      (Physics|SetSimulatePhysics CableHitComponent true))))

(fn SetCableHitVariables
  (params (CableHitDistance :type Float%20%28single-precision%29) (CableHitActor :type Actor%20Object%20Reference) (CableHitComponent :type Primitive%20Component%20Object%20Reference) (CableHitBoneName :type Name))
  (Variables|Default|SetCableHitComponent CableHitComponent)
  (Variables|Default|SetCableHitActor CableHitActor)
  (Variables|Default|SetCableHitBoneName CableHitBoneName)
  (Variables|Default|SetCableHitDistance CableHitDistance))

(fn CheckHitActorisEnemy
  (return (== (Utilities|GetClass (Variables|Default|GetCableHitActor)) "/Game/Enemy/EnemyPH_BP.EnemyPH_BP_C")))