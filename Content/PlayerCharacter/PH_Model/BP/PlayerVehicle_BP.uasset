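; Player-controlled hover vehicle pawn that handles movement, boosting, aiming, shooting and shielded health.
; Interface input applies physics forces along control yaw, swaps first- and third-person cameras, and forwards firing to a socket-attached weapon.
; Tick interpolates mesh yaw toward the active camera, adding pitch when airborne.
; Damage drains shield before health, restarts a delayed looping regeneration timer, and destroys the vehicle when health runs out with the shield down.
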(event Custom|OnTakeAnyDamage_Event
  (params (DamagedActor :type Actor%20Object%20Reference) (Damage :type Float%20%28single-precision%29) (DamageType :type Damage%20Type%20Object%20Reference) (InstigatedBy :type Controller%20Object%20Reference) (DamageCauser :type Actor%20Object%20Reference))
  (CallFunction|CalculateTakenDamage Damage)
  ;[1 1 1] Set timer for shield regen so when hit again it resets the intial start delay
  (bind _returnvalue (Utilities|Time|SetTimerbyEvent (delegate Custom|ShieldRegenerationEvent) (Variables|Default|GetShieldRegenCooldownTick) true (Variables|Default|GetShieldRegenCooldownStart))))

(event Custom|OnDeath
  (params (DestroyedActor :type Actor%20Object%20Reference))
  (Class|Pawn|DetachfromControllerPendingDestroy))

(event Custom|ShieldRegenerationEvent
  (bind _maxshield (Variables|Default|GetMaxShield))
  (if (>= _maxshield (Variables|Default|GetShield))
    ;[1 1 1] Regen shields
    (bind _output_get (Variables|Default|SetShield (+ (Variables|Default|GetShield) (Variables|Default|GetShieldRegenAmount))))
    ;[1 1 1] Check if there is any shield so damage taken will be taken from the shield not HP
    (if (> _output_get 0.0)
      (Variables|Default|SetisShieldDown false))
    (else
      ;[1 1 1] Set shield to max and pause timer to not loop it
      (Variables|Default|SetShield _maxshield)
      (Utilities|Time|ClearandInvalidateTimerbyHandle (stale Custom|OnTakeAnyDamage_Event _returnvalue)))))

(event EventBeginPlay
  (EventDispatchers|BindEventtoOnTakeAnyDamage (delegate Custom|OnTakeAnyDamage_Event))
  (Game|BindEventtoOnDestroyed (delegate Custom|OnDeath))
  (Variables|Default|SetActiveCamera (Variables|Default|GetThirdPersonCamera)))

(event EventTick
  (params (DeltaSeconds :type Float%20%28single-precision%29))
  (bind _returnvalue (Utilities|Time|GetWorldDeltaSeconds))
  (bind _defaultinterpspeed (Variables|Default|GetDefaultInterpSpeed))
  (bind _activecamera (Variables|Default|GetActiveCamera))
  (bind _vehiclemesh (Variables|Default|GetVehicleMesh))
  (bind _returnvalue_2 (Transformation|GetWorldRotation _activecamera))
  (bind _returnvalue_3 (Transformation|GetWorldRotation _vehiclemesh))
  (bind (_roll _pitch) (Math|Rotator|BreakRotator _returnvalue_3))
  (bind _returnvalue_4 (Math|Interpolation|RInterpTo _returnvalue_3 (Math|Rotator|MakeRotator (.roll _returnvalue_2) (.pitch _returnvalue_2) (.yaw _returnvalue_2)) _returnvalue _defaultinterpspeed))
  ;[1 1 1] Set mesh to rotate related to camera
  ;;[1 1 1] If even one of hover component's line trace hits something this is true
  (if (Variables|Default|GetisOnGround)
    (Transformation|SetWorldRotation (Variables|Default|GetVehicleMesh) (Math|Rotator|MakeRotator _roll _pitch (.yaw _returnvalue_4)) false true)
    (else
      (Transformation|SetWorldRotation (Variables|Default|GetVehicleMesh) (Math|Rotator|MakeRotator _roll (.pitch _returnvalue_4) (.yaw _returnvalue_4)) false true))))

(event EventPlayerMovement
  (params (InputValue :type Vector%202D%20Structure))
  ;[1 1 1] Handle player movement with PlayerInput_BPI Blueprint interface
  (CallFunction|CalculateForwardForce (.x InputValue))
  (CallFunction|CalculateStrafeForce (.y InputValue)))

(event EventPlayerShoot
  (bind _weaponref (Variables|Default|GetWeaponRef))
  ;[1 1 1] Handle shooting action with BPI and call the event on attached weapon component
  (Utilities|IsValid _weaponref
    (:Is%20Valid
      (Default|PlayerShoot _weaponref))))

(event EventPlayerBoost
  (params (isBoostOn :type Boolean))
  ;[1 1 1] Handle boost action with Player Movement BPI
  (if isBoostOn
    ;;[1 1 1] Call this when boosting happens
    (Variables|Default|SetForwardForce (Variables|Default|GetFowardForceBoost))
    (Variables|Default|SetDefaultInterpSpeed (Variables|Default|GetInterpSpeedMax))
    (else
      ;;[1 1 1] Call this to return normal speed
      (Variables|Default|SetForwardForce (Variables|Default|GetForwardForceDefault))
      (Variables|Default|SetDefaultInterpSpeed (Variables|Default|GetInterpSpeedMin)))))

(event EventPlayerAim
  (params (isAiming :type Boolean))
  (if isAiming
    (Components|Activation|SetActive (Variables|Default|GetFirstPersonCamera) true false)
    (Components|Activation|SetActive (Variables|Default|GetThirdPersonCamera) false false)
    (Variables|Default|SetActiveCamera (Variables|Default|GetFirstPersonCamera))
    (else
      (Components|Activation|SetActive (Variables|Default|GetThirdPersonCamera) true false)
      (Components|Activation|SetActive (Variables|Default|GetFirstPersonCamera) false false)
      (Variables|Default|SetActiveCamera (Variables|Default|GetThirdPersonCamera)))))

(fn ConstructionScript)

(fn CalculateTakenDamage
  (params (Damage :type Float%20%28double-precision%29))
  (if (Variables|Default|GetisShieldDown)
    (bind _output_get (Variables|Default|SetHealth (- (Variables|Default|GetHealth) Damage)))
    (Development|PrintString (Utilities|String|ToString(Float) _output_get) true true "(R=1.000000,G=0.000000,B=0.016606,A=1.000000)")
    (if (<= _output_get 0.0)
      (Actor|DestroyActor))
    (elif (> (Variables|Default|GetShield) Damage)
      ;[1 1 1] Shield - Damage
      (bind _output_get_2 (Variables|Default|SetShield (- (Variables|Default|GetShield) Damage)))
      (Development|PrintString (Utilities|String|ToString(Float) _output_get_2))
      (else
        ;[1 1 1] If damage is greater than current shield take health damage from that damage is left
        (Variables|Default|SetShield 0.0)
        (Variables|Default|SetisShieldDown true)
        (bind _output_get_3 (Variables|Default|SetHealth (- (Variables|Default|GetHealth) (- Damage (Variables|Default|GetShield)))))
        (Development|PrintString (Utilities|String|ToString(Float) _output_get_3))))))

(fn CalculateForwardForce
  (params (InputValue :type Float%20%28double-precision%29))
  (Physics|AddForce (Variables|Default|GetVehicleMesh) (* (* (Math|Vector|GetForwardVector (Math|Rotator|MakeRotator 0.0 0.0 (.yaw (Pawn|GetControlRotation :!class /Script/Engine.Pawn)))) (* (Variables|Default|GetForwardForce) (Variables|Default|GetForceMultiplier))) InputValue) "None" false))

(fn CalculateStrafeForce
  (params (InputValue :type Float%20%28double-precision%29))
  (Physics|AddForce (Variables|Default|GetVehicleMesh) (* (* (Math|Vector|GetRightVector (Math|Rotator|MakeRotator 0.0 0.0 (.yaw (Pawn|GetControlRotation :!class /Script/Engine.Pawn)))) (* (Variables|Default|GetRightForce) (Variables|Default|GetForceMultiplier))) InputValue) "None" false))

(fn AddWeapon
  (Utilities|IsValid (Variables|Default|GetWeaponRef)
    (:Is%20Not%20Valid
      (bind _returnvalue (Game|SpawnActorfromClass "/Game/WP_PH/BP/Weapon_BP.Weapon_BP_C" (Transformation|GetSocketTransform (Variables|Default|GetVehicleMesh) "Weapon_Socket" "RTS_Component") "AlwaysSpawn" self 0))
      (Transformation|AttachComponentToComponent _returnvalue (Variables|Default|GetVehicleMesh) "Weapon_Socket" "SnapToTarget" "SnapToTarget" "SnapToTarget" true)
      (Variables|Default|SetWeaponRef _returnvalue))))