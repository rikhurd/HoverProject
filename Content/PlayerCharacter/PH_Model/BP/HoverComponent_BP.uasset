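; Hover suspension component that pushes its owner's skeletal mesh away from the surface below, acting as one spring-damper point.
; Each tick it line-traces along its negative up vector on the Visibility channel, with debug drawing on.
; On a hit, a spring force from compression and its rate of change is applied along the surface normal at the component's location.
; Hits also set the mesh's linear and angular damping, which is never reset on a miss.
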(event EventBeginPlay
  (Variables|Default|SetParentComponent (Actor|GetComponentbyClass (Components|GetOwner) "/Script/Engine.SkeletalMeshComponent")))

(event EventTick
  (params (DeltaSeconds :type Float%20%28single-precision%29))
  (bind _returnvalue (Transformation|GetWorldLocation))
  (bind _parentcomponent (Variables|Default|GetParentComponent))
  (bind (_outhit _returnvalue_2) (Collision|LineTraceByChannel _returnvalue (- _returnvalue (* (Math|Vector|GetUpVector) (Variables|Default|GetTraceLength))) "TraceTypeQuery1" false 0 "ForOneFrame"))
  (if _returnvalue_2
    (Class|PrimitiveComponent|AddForceatLocation _parentcomponent (CallFunction|CalculateSpringForce (.Distance (Collision|BreakHitResult _outhit)) (.Normal (Collision|BreakHitResult _outhit))) (Transformation|GetWorldLocation) "None")
    (Class|PrimitiveComponent|SetLinearDamping _parentcomponent (Variables|Default|GetLinearDamping))
    (Class|PrimitiveComponent|SetAngularDamping _parentcomponent (Variables|Default|GetAngularDamping))
    (Variables|Default|SetSuspensionPrevious (Variables|Default|GetSuspensionDelta))))

(fn CalculateSpringForce
  (params (Distance :type Float%20%28double-precision%29) (Normal :type Vector))
  (Variables|Default|SetSuspensionDelta (- (Variables|Default|GetTraceLength) Distance))
  (return (* Normal (* (+ (* (Variables|Default|GetSuspensionDelta) (Variables|Default|GetStiffness)) (* (/ (- (Variables|Default|GetSuspensionDelta) (Variables|Default|GetSuspensionPrevious)) (Utilities|Time|GetWorldDeltaSeconds)) (Variables|Default|GetDamping))) (Variables|Default|GetHoverForce)))))